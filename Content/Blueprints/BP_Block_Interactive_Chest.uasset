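; BP_Block_Interactive_Chest is an interactive chest block whose lid opens and closes on alternate interactions.
; On BeginPlay it copies the Block mesh's first material onto the chest top mesh.
; Interact uses a FlipFlop to play or reverse the OpenChest timeline, whose ChestOpen track drives the pitch of the PivotEmpty component.
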(event `self.ReceiveBeginPlay`
  (`parent.ReceiveBeginPlay`)
  (`PrimitiveComponent.SetMaterial` (`self.SM_Chest_Top`) 0 (`PrimitiveComponent.GetMaterial` (`self.Block`) 0)))

(event `self.Interact`
  (`/Engine/EditorBlueprintResources/StandardMacros.FlipFlop`
    (:`A`
      (bind (_direction _chestopen) (`Timeline|OpenChest` :!label _label)
        (:`Update`
          (`SceneComponent.K2_SetRelativeRotation` (`self.Pivot Empty`) (`KismetMathLibrary.MakeRotator` 0.0 _chestopen) false false))))
    (:`B`
      (goto _label :!via `Reverse`))))

(fn `UserConstructionScript`
  (`parent.UserConstructionScript`))